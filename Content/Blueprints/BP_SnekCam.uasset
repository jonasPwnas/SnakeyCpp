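; BP_SnekCam is a camera Blueprint for a two-player snake game that selects the leading player as its tracking target.
; After a startup delay, it caches the camera's starting rotations and game mode, sorts both pawns by player index, then enables Tick.
; Each Tick calls the parent, then sets TrackTarget to the higher scorer, or None on a tie.
; No live node here rotates the camera.
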(event `self.ReceiveBeginPlay`
  (bind _camera (`self.Camera`))
  (`KismetSystemLibrary.Delay` 3.0)
  (set `self.StartWorldRotation` (`SceneComponent.K2_GetComponentRotation` _camera))
  (set `self.StartRelativeRotation` (`SceneComponent.RelativeRotation` _camera))
  (bind _assnake_game_mode (cast `SnakeGameMode` (`GameplayStatics.GetGameMode`)))
  (set `self.As Snake Game Mode` _assnake_game_mode)
  (bind _assnake_player (cast `SnakePlayer` (`PlayerState.GetPawn` (`|GetArrayItem` (`GameStateBase.PlayerArray` (`GameplayStatics.GetGameState`))))))
  (if (== (`SnakePlayer.SnekPlayerIndex` _assnake_player) 0)
    (set `self.Player1` _assnake_player)
    (else
      (set `self.Player2` _assnake_player)))
  (bind _assnake_player_2 (cast `SnakePlayer` (`PlayerState.GetPawn` (`|GetArrayItem` (`GameStateBase.PlayerArray` (`GameplayStatics.GetGameState`)) 1))))
  (if (== (`SnakePlayer.SnekPlayerIndex` _assnake_player_2) 0)
    (set `self.Player1` _assnake_player_2)
    (else
      (set `self.Player2` _assnake_player_2)))
  (`self.SetActorTickEnabled` true))

(event `self.ReceiveTick`
  (params (DeltaSeconds :type "Float (single-precision)"))
  (bind _as_snake_game_mode (`self.As Snake Game Mode`))
  (bind _player1score (`SnakeGameMode.Player1Score` _as_snake_game_mode))
  (bind _player2score (`SnakeGameMode.Player2Score` _as_snake_game_mode))
  (`parent.ReceiveTick` DeltaSeconds)
  (if (== _player1score _player2score)
    (set `self.TrackTarget` null)
    (else
      (set `self.TrackTarget` (select `bool` (> _player1score _player2score) :`false` (`self.Player2`) :`true` (`self.Player1`) :!type "Actor Object Reference")))))

(fn `UserConstructionScript`)