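; BP_SnekMode2 is the game mode for a two-player Snek match, creating the level 2 HUD for countdown, scores and winner display.
; Growth events raise that player's score, and reaching WinningScore shows them as winner and kills the other snake.
; A once-only death handler spawns an explosion, declares the survivor winner, hides the dead snake, halts movement on all snakes and switches input to include UI.
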(event `self.ReceiveBeginPlay`
  (bind _returnvalue (`GameplayStatics.GetPlayerController` 0))
  (`parent.ReceiveBeginPlay`)
  (add `self.OnCountdownChanged` (delegate `NewCount`))
  (add `self.OnStart` (delegate `GameStart`))
  (add `self.OnReachedMaxScore` (delegate `OnWinner`))
  (bind _returnvalue_2 (`|CreateWidget` "/Game/Widgets/WBP_Lvl2Hud.WBP_Lvl2Hud_C"))
  (set `self.HudRef` _returnvalue_2)
  (`UserWidget.AddToViewport` _returnvalue_2 0)
  (`WidgetBlueprintLibrary.SetInputMode_GameOnly` _returnvalue)
  (set `PlayerController.bShowMouseCursor` false _returnvalue))

(event `NewCount` :!signature `self.OnCountdownChanged`
  (params (NewCount :type Integer))
  (`/Game/Widgets/WBP_SharedHud.SetCountdown` (`self.HudRef`) (`KismetTextLibrary.Conv_IntToText` NewCount)))

(event `GameStart` :!signature `self.OnStart`
  (params (bStartSession :type Boolean))
  (`/Game/Widgets/WBP_SharedHud.HideCountDown` (`self.HudRef`)))

(event `OnWinner` :!signature `self.OnReachedMaxScore`
  (params (WinnerPlayer :type "SnakePlayer Object Reference"))
  (`/Game/Widgets/WBP_SharedHud.ShowWinnerWidget` (`self.HudRef`) (`KismetTextLibrary.Conv_IntToText` (`SnakePlayer.SnekPlayerIndex` WinnerPlayer))))

(event `self.SomeoneDiedOhNo`
  (params (Player :type "SnakePlayer Object Reference"))
  (bind _returnvalue (`GameplayStatics.GetPlayerController` 0))
  (bind _hudref (`self.HudRef`))
  (`/Engine/EditorBlueprintResources/StandardMacros.DoOnce` false
    (:`Completed`
      (`NiagaraFunctionLibrary.SpawnSystemAtLocation` "/Game/MixedVFX/Particles/Explosions/NS_ExplosionGroundBig.NS_ExplosionGroundBig" (`self.K2_GetActorLocation` Player))
      (`/Game/Widgets/WBP_SharedHud.ShowWinnerWidget` _hudref (`KismetTextLibrary.Conv_IntToText` (`KismetMathLibrary.SelectInt` 2 1 (== (`SnakePlayer.SnekPlayerIndex` Player) 0))))
      (`WidgetBlueprintLibrary.SetInputMode_GameAndUIEx` _returnvalue _hudref)
      (set `PlayerController.bShowMouseCursor` true _returnvalue)
      (`self.SetActorHiddenInGame` Player true)
      (`self.SetActorEnableCollision` Player false)
      ; not great but, it works :')
      (bind _outactors (`GameplayStatics.GetAllActorsOfClass` "/Game/Blueprints/BP_SnakePlayer.BP_SnakePlayer_C"))
      (for _array_element _outactors
        (set `SnakePlayer.bCanMove` false _array_element))
      (`self.OnStart` false))))

(event `self.SomeoneGrewOhYes`
  (params (Player :type "SnakePlayer Object Reference"))
  (bind _hudref (`self.HudRef`))
  (bind _player1score (`self.Player1Score`))
  (bind _player2score (`self.Player2Score`))
  (if (== (`SnakePlayer.SnekPlayerIndex` Player) 0)
    (bind _output_get (set `self.Player1Score` (+ _player1score 1)))
    (`/Game/Widgets/WBP_SharedHud.SetP1Score` _hudref (`KismetTextLibrary.Conv_IntToText` _output_get))
    (if (>= _player1score (`self.WinningScore`))
      (`/Game/Widgets/WBP_SharedHud.ShowWinnerWidget` (`self.HudRef`) "1")
      (bind _outactors (`GameplayStatics.GetAllActorsOfClass` "/Game/Blueprints/BP_SnakePlayer.BP_SnakePlayer_C"))
      (for _array_element _outactors
        (if (== (`SnakePlayer.SnekPlayerIndex` _array_element) 1)
          (`SnakePlayer.Die` _array_element))))
    (else
      (bind _output_get_2 (set `self.Player2Score` (+ _player2score 1)))
      (`/Game/Widgets/WBP_SharedHud.SetP2Score` _hudref (`KismetTextLibrary.Conv_IntToText` _output_get_2))
      (if (>= _player2score (`self.WinningScore`))
        (`/Game/Widgets/WBP_SharedHud.ShowWinnerWidget` (`self.HudRef`) "2")
        (bind _outactors_2 (`GameplayStatics.GetAllActorsOfClass` "/Game/Blueprints/BP_SnakePlayer.BP_SnakePlayer_C"))
        (for _array_element_2 _outactors_2
          (if (== (`SnakePlayer.SnekPlayerIndex` _array_element_2) 0)
            (`SnakePlayer.Die` _array_element_2)))))))

(fn `UserConstructionScript`)